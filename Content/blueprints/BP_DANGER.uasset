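; BP_DANGER is a moving hazard that damages the player character on contact.
; Its construction script gives an InterpToMovement component two relative control points, the origin and MoveToPos, so each instance gets its own path.
; When the trigger overlaps a BP_ThirdPersonCharacter1, it applies damage, spawns a fire burst at the character and plays a 2D hit sound, destroying the emitter after a short delay.
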(event OnComponentBeginOverlap(trigger)
  (params (OverlappedComponent :type Primitive%20Component%20Object%20Reference) (OtherActor :type Actor%20Object%20Reference) (OtherComp :type Primitive%20Component%20Object%20Reference) (OtherBodyIndex :type Integer) (bFromSweep :type Boolean) (SweepResult :type Hit%20Result%20Structure%20%28by%20ref%29))
  (bind _asbp_third_person_character_1 (Utilities|Casting|CastToBP_ThirdPersonCharacter1 OtherActor))
  (Default|TakeDamage _asbp_third_person_character_1 25.0)
  (bind _returnvalue (Effects|SpawnEmitteratLocation "/Game/InfinityBladeEffects/Effects/FX_Forging/P_StamperFireBurst.P_StamperFireBurst" (Transformation|GetActorLocation _asbp_third_person_character_1)))
  (Audio|PlaySound2D "/Game/sounds/video-game-hit-noise-001-135821.video-game-hit-noise-001-135821" 1.0 1.0 0.0 0 0)
  (Utilities|FlowControl|Delay 2.0)
  (Components|DestroyComponent _returnvalue))

(fn ConstructionScript
  (Class|InterptoMovementComponent|AddControlPointPosition (Variables|Default|GetInterpToMovement) "0, 0, 0" true)
  (Class|InterptoMovementComponent|AddControlPointPosition (Variables|Default|GetInterpToMovement) (Variables|Default|GetmoveToPos) true))