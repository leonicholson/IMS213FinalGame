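; BP_collectableFish is a collectable fish pickup that increments the player character's fish count.
; Each tick it spins the FishLowPoly component in yaw by RotationSpeed, with no delta-time scaling.
; When PickupRadius is overlapped, it casts the other actor's instigator to BP_ThirdPersonCharacter1, adds one to Fishes and plays a 2D chomp sound.
; It destroys itself after a short delay, with no guard against repeat overlaps meanwhile.
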(event OnComponentBeginOverlap(pickupRadius)
  (params (OverlappedComponent :type Primitive%20Component%20Object%20Reference) (OtherActor :type Actor%20Object%20Reference) (OtherComp :type Primitive%20Component%20Object%20Reference) (OtherBodyIndex :type Integer) (bFromSweep :type Boolean) (SweepResult :type Hit%20Result%20Structure%20%28by%20ref%29))
  (bind _asbp_third_person_character_1 (Utilities|Casting|CastToBP_ThirdPersonCharacter1 (Game|GetInstigator OtherActor)))
  (Variables|/Game/ThirdPerson/Blueprints/BP_ThirdPersonCharacter1.BP_ThirdPersonCharacter1_C|Setfishes _asbp_third_person_character_1 (+ (Variables|/Game/ThirdPerson/Blueprints/BP_ThirdPersonCharacter1.BP_ThirdPersonCharacter1_C|Getfishes _asbp_third_person_character_1) 1))
  (Audio|PlaySound2D "/Game/sounds/chomp-1.chomp-1" 1.0 1.0 0.0 0 0)
  (Utilities|FlowControl|Delay 0.2)
  (Actor|DestroyActor))

(event EventTick
  (params (DeltaSeconds :type Float%20%28single-precision%29))
  ;[1 1 1] rotating fish
  (Transformation|AddRelativeRotation (Variables|Default|Getfish_low_poly) (Math|Rotator|MakeRotator 0.0 0.0 (Variables|Default|Getrotation%20speed)) false false))

(fn ConstructionScript)