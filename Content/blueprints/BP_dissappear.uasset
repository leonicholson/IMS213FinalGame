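; Disappearing brick platform that vanishes shortly after the third-person player character touches its trigger box.
; Box overlap begin turns the brick white, then after a short delay hides it and disables its collision.
; Overlap end waits longer, then restores the grey material, visibility and collision, without checking which actor left.
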(event OnComponentBeginOverlap(Box)
  (params (OverlappedComponent :type Primitive%20Component%20Object%20Reference) (OtherActor :type Actor%20Object%20Reference) (OtherComp :type Primitive%20Component%20Object%20Reference) (OtherBodyIndex :type Integer) (bFromSweep :type Boolean) (SweepResult :type Hit%20Result%20Structure%20%28by%20ref%29))
  (Utilities|Casting|CastToBP_ThirdPersonCharacter1 OtherActor)
  (Rendering|Material|SetMaterial (Variables|Default|GetdissapearBrick) 0 "/Game/models/platforms/White.White")
  (Utilities|FlowControl|Delay 0.5)
  (Rendering|SetVisibility (Variables|Default|GetdissapearBrick) false false)
  (Collision|SetCollisionEnabled (Variables|Default|GetdissapearBrick) "NoCollision"))

(event OnComponentEndOverlap(Box)
  (params (OverlappedComponent :type Primitive%20Component%20Object%20Reference) (OtherActor :type Actor%20Object%20Reference) (OtherComp :type Primitive%20Component%20Object%20Reference) (OtherBodyIndex :type Integer))
  (Utilities|FlowControl|Delay 2.0)
  (Rendering|Material|SetMaterial (Variables|Default|GetdissapearBrick) 0 "/Game/models/platforms/Grey_001.Grey_001")
  (Rendering|SetVisibility (Variables|Default|GetdissapearBrick) true false)
  (Collision|SetCollisionEnabled (Variables|Default|GetdissapearBrick) "QueryAndPhysics"))

(event EventBeginPlay)

(event Collision|EventActorBeginOverlap
  (params (OtherActor :type Actor%20Object%20Reference)))

(event EventTick
  (params (DeltaSeconds :type Float%20%28single-precision%29)))

(fn ConstructionScript)